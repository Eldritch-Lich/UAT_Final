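; LaunchDetector is a projectile that tests whether it strikes a Targetable_Cube and records a point to launch the player to.
; A valid hit stores the location and cube, flags the target as valid and calls Targetted on the cube.
; After UseTime it enables mesh gravity and stops counting as valid.
; Every hit sets a lifespan, five times longer when a still-valid shot hits something else.
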(event EventBeginPlay
  (Utilities|FlowControl|Delay (Variables|Default|GetUseTime))
  (Physics|SetEnableGravity (Variables|Default|GetStaticMesh) true)
  (Variables|Default|SetValidProjectile false))

(event Collision|EventHit
  (params (MyComp :type Primitive%20Component%20Object%20Reference) (Other :type Actor%20Object%20Reference) (OtherComp :type Primitive%20Component%20Object%20Reference) (bSelfMoved :type Boolean) (HitLocation :type Vector :default "0, 0, 0") (HitNormal :type Vector :default "0, 0, 0") (NormalImpulse :type Vector :default "0, 0, 0") (Hit :type Hit%20Result%20Structure%20%28by%20ref%29))
  (if (Variables|Default|GetValidProjectile)
    (if (== (Utilities|GetClass Other) "/Game/MyAssets/Blueprints/Targetable_Cube.Targetable_Cube_C")
      (Variables|Default|SetValidTarget true)
      (Variables|Default|SetLaunchPlayerHere HitLocation)
      (Development|PrintString "IsTCube")
      (Actor|SetLifeSpan (Variables|Default|GetLifeSpan))
      (bind _astargetable_cube (Utilities|Casting|CastToTargetable_Cube Other))
      (Default|Targetted _astargetable_cube)
      (Variables|Default|SetAs%20Targetable%20Cube _astargetable_cube)
      (else
        (Variables|Default|SetValidTarget false)
        (Development|PrintString "NotTCube")
        (Actor|SetLifeSpan (* (Variables|Default|GetLifeSpan) 5.0))))
    (else
      (Actor|SetLifeSpan (Variables|Default|GetLifeSpan)))))

(fn ConstructionScript)

(fn GetHitLocation
  (params (HitLocation :type Vector))
  (return HitLocation))