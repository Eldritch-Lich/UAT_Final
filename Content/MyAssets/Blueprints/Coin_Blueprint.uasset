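; Collectible coin that destroys itself on player overlap, then notifies CustomGamemode and plays a sound.
; After a random startup delay, it picks a random spin speed and direction, then enables Tick.
; Tick spins it and moves it toward cached upper or lower targets, using Delays to toggle direction.
; MakeLight also runs once at startup, spawning a Targetable_Cube between the coin and a nearby VertDeath actor, if found.
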(event EventBeginPlay
  (bind _rotmax (Variables|Default|GetRotMax))
  (bind _rotmin (Variables|Default|GetRotMin))
  (bind _returnvalue (Math|Random|RandomFloatinRange _rotmin _rotmax))
  (CallFunction|GetFloatVectors)
  (Actor|Tick|SetActorTickEnabled false)
  (Utilities|FlowControl|Delay (Math|Random|RandomFloat))
  (Utilities|FlowControl|Sequence
    (:then_0
      (bind _output_get (Variables|Default|SetRotationSpeed _returnvalue))
      (for _index (range 0 (Math|Float|Truncate _returnvalue))
        (Utilities|FlowControl|FlipFlop
          (:A
            (Variables|Default|SetRotationSpeed (* _output_get -1.0))
            (Actor|Tick|SetActorTickEnabled true))
          (:B
            (Actor|Tick|SetActorTickEnabled true)))))
    (:then_1
      (CallFunction|MakeLight))))

(event EventTick
  (params (DeltaSeconds :type Float%20%28single-precision%29))
  (bind _duration (Variables|Default|GetDuration))
  (Utilities|FlowControl|Delay DeltaSeconds)
  (Transformation|AddActorLocalRotation (Math|Rotator|MakeRotator 0.0 0.0 (Variables|Default|GetRotationSpeed)) false false)
  (if (Variables|Default|GetUpDown)
    (bind _normalizedvector (CallFunction|CalculateVectorMovement (Variables|Default|GetUpperVectorTarget)))
    (CallFunction|MoveActorbyVector _normalizedvector 0.0)
    (Utilities|FlowControl|Delay _duration)
    (Variables|Default|SetUpDown false)
    (else
      (bind _normalizedvector_2 (CallFunction|CalculateVectorMovement (Variables|Default|GetLowerVectorTarget)))
      (CallFunction|MoveActorbyVector _normalizedvector_2 0.0)
      (Utilities|FlowControl|Delay _duration)
      (Variables|Default|SetUpDown true))))

(event Collision|EventActorBeginOverlap
  (params (OtherActor :type Actor%20Object%20Reference))
  (if (== OtherActor (Game|Player|GetPlayerPawn 0))
    (Actor|DestroyActor)))

(event EventDestroyed
  (bind _ascustom_gamemode (Utilities|Casting|CastToCustomGamemode (Game|GetGameMode)))
  (Default|CoinCollected _ascustom_gamemode)
  (Audio|SpawnSound2D "/Game/MyAssets/Sounds/Weird_Coin.Weird_Coin" 1.0 1.0 0.0 0))

(fn ConstructionScript)

(fn GetFloatVectors
  (Variables|Default|SetUpperVectorTarget (Transformation|GetSocketLocation (Variables|Default|GetUpperTarget) "None"))
  (Variables|Default|SetLowerVectorTarget (Transformation|GetSocketLocation (Variables|Default|GetLowerTarget) "None")))

(fn CalculateVectorMovement
  (params (VectorDestination :type Vector))
  (return (Math|Vector|Normalize (- VectorDestination (Transformation|GetActorLocation)))))

(fn MoveActorbyVector
  (params (VectorDirection :type Vector) (SecondLimiter :type Float%20%28double-precision%29))
  (Transformation|SetActorLocation (+ (Transformation|GetActorLocation) (* VectorDirection (Variables|Default|GetFloatSpeed))) false false))

(fn MakeLight
  (bind _outactors (Collision|SphereOverlapActors (Transformation|GetActorLocation) 3e+02 (Variables|Default|GetObject%20Types) "/Game/MyAssets/Blueprints/VertDeath.VertDeath_C"))
  (bind _output_get (LocalVariables|SetNearbyHorizDeaths _outactors))
  (if (Utilities|IsValid (Utilities|Array|Get(acopy) _output_get))
    (Game|SpawnActorfromClass "/Game/MyAssets/Blueprints/Targetable_Cube.Targetable_Cube_C" (Math|Conversions|ToTransform(Vector) (/ (+ (Transformation|GetActorLocation) (Transformation|GetActorLocation (Utilities|Array|Get(acopy) _output_get))) (LocalVariables|GetDivideBy))) "Undefined" 0 0)
    (Development|PrintString "Spawned")
    (else
      (Development|PrintString "Invalid Objects"))))