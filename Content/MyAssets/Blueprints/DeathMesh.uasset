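; DeathMesh is a hazard actor that kills the player on contact and records the death.
; Its Hit event checks whether the other actor is the first player pawn, then has its KillComponent deactivate the player.
; It then increments the death counter on the CustomGameInstance and prints a "Death" message.
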(event Custom|IncrementDeathCounter
  (bind _ascustom_game_instance (Utilities|Casting|CastToCustomGameInstance (Game|GetGameInstance)))
  (Default|IncrementDeaths _ascustom_game_instance)
  (Development|PrintString "Death"))

(event Collision|EventHit
  (params (MyComp :type Primitive%20Component%20Object%20Reference) (Other :type Actor%20Object%20Reference) (OtherComp :type Primitive%20Component%20Object%20Reference) (bSelfMoved :type Boolean) (HitLocation :type Vector :default "0, 0, 0") (HitNormal :type Vector :default "0, 0, 0") (NormalImpulse :type Vector :default "0, 0, 0") (Hit :type Hit%20Result%20Structure%20%28by%20ref%29))
  (bind _playertrue (CallFunction|CheckPlayerContact Other))
  (if _playertrue
    (Default|DeactivatePlayer (Variables|Default|GetKillComponent))
    (CallFunction|IncrementDeathCounter)))

(fn ConstructionScript)

(fn CheckPlayerContact
  (params (OtherObject :type Object%20Object%20Reference))
  (return (== OtherObject (Game|Player|GetPlayerPawn 0))))