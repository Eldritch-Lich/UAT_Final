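; Launched_Cube is an actor that fires a LaunchDetector projectile from its LaunchDirection component two seconds after play begins.
; The direction is the normalized vector from the actor's location to the LaunchDirection component, captured at BeginPlay before the delay.
; The spawned detector's mesh has gravity off and physics on, then gets a velocity-change impulse scaled by DetectionSpeed, so it flies straight regardless of mass.
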(event EventBeginPlay
  (bind _directionvector (CallFunction|GetDirectionVector))
  (Utilities|FlowControl|Delay 2.0)
  (bind _returnvalue (Game|SpawnActorfromClass "/Game/MyAssets/Blueprints/LaunchDetector.LaunchDetector_C" (Math|Conversions|ToTransform(Vector) (Transformation|GetSocketLocation (Variables|Default|GetLaunchDirection) "None")) "Undefined" 0 0))
  (Physics|SetEnableGravity (Variables|/Game/MyAssets/Blueprints/LaunchDetector.LaunchDetector_C|GetStaticMesh _returnvalue) false)
  (Physics|SetSimulatePhysics (Variables|/Game/MyAssets/Blueprints/LaunchDetector.LaunchDetector_C|GetStaticMesh _returnvalue) true)
  (Physics|AddImpulse (Variables|/Game/MyAssets/Blueprints/LaunchDetector.LaunchDetector_C|GetStaticMesh _returnvalue) (* _directionvector (Variables|Default|GetDetectionSpeed)) "None" true))

(fn ConstructionScript)

(fn GetDirectionVector
  (return (Math|Vector|Normalize (- (Transformation|GetSocketLocation (Variables|Default|GetLaunchDirection) "None") (Transformation|GetActorLocation)))))